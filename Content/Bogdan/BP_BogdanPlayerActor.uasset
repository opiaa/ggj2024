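; BP_BogdanPlayerActor is a possessable player pawn that appears to be a test of local multiplayer control and input.
; On BeginPlay it gets the player controller at MyCharacterControllerIndex, creating a local player if none exists, and has it possess this pawn.
; It then adds the IMC_Default Enhanced Input mapping context to that controller.
; Possession, gamepad move input and a G debug key only print debug names, with no movement logic.
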(event Input|EnhancedActionEvents|EnhancedInputActionMove_Gamepad
  (params (ActionValue :type Vector%202D%20Structure) (ElapsedSeconds :type Float%20%28double-precision%29) (TriggeredSeconds :type Float%20%28double-precision%29) (InputAction :type Input%20Action%20Object%20Reference :default "/Game/TopDown/Input/Actions/Move_Gamepad.Move_Gamepad"))
  (:Triggered
    (Development|PrintString (Utilities|GetObjectName self) :!label _label))
  (:Started
    (goto _label))
  (:Ongoing
    (goto _label)))

(event EventBeginPlay
  (bind _self self)
  (bind _mycharactercontrollerindex (Variables|Default|GetMyCharacterControllerIndex))
  (bind _returnvalue (Game|GetPlayerController _mycharactercontrollerindex))
  (Utilities|IsValid _returnvalue
    (:Is%20Valid
      (Pawn|Possess _returnvalue _self))
    (:Is%20Not%20Valid
      (bind _returnvalue_2 (Class|GameplayStatics|CreatePlayer _mycharactercontrollerindex))
      (Pawn|Possess _returnvalue_2 _self)))
  (Input|AddMappingContext (PlayerController|LocalPlayerSubsystems|GetEnhancedInputLocalPlayerSubsystem (Game|GetPlayerController (Variables|Default|GetMyCharacterControllerIndex))) "/Game/TopDown/Input/IMC_Default.IMC_Default" 0 (Utilities|Struct|MakeModifyContextOptions true false false)))

(event Collision|EventActorBeginOverlap
  (params (OtherActor :type Actor%20Object%20Reference)))

(event EventTick
  (params (DeltaSeconds :type Float%20%28single-precision%29)))

(event EventPossessed
  (params (NewController :type Controller%20Object%20Reference))
  (Development|PrintString (Utilities|String|ToString(Text) (Utilities|Text|FormatText "{b} Possessed by {a}" (Utilities|GetObjectName NewController) (Utilities|GetObjectName self)))))

(event Input|KeyboardEvents|DebugKeyG
  (params (Key :type Key%20Structure :default "None") (ActionValue :type Input%20Action%20Value%20Structure))
  (:Pressed
    (Development|PrintString (Utilities|GetObjectName self))))

(fn ConstructionScript)