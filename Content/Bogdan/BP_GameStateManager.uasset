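; BP_GameStateManager runs the game flow through intro, match and scoring states, with short waiting states that cover fade-outs.
; Setup places players on podiums with menu music; match start teleports them to player starts and begins voice-system music, and match end swaps it for the win song.
; Tick blends to the podium or arena camera, shows the intro widget only during Intro, and spring-interpolates a post-process collection fade parameter.
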(event Custom|DoFade
  (Variables|Default|SetFadeTarget 1.0))

(event Custom|ClearFade
  (Variables|Default|SetFadeTarget 0.0))

(event Custom|BeginAfterDelay
  (Utilities|FlowControl|Delay 1.0)
  (Variables|Default|SetFadeTarget 0.0)
  (bind _returnvalue (Actor|GetActorOfClass "/Game/Bogdan/BP_VoiceSystem.BP_VoiceSystem_C"))
  (Default|BeginMusic _returnvalue)
  (Variables|Default|SetState "NewEnumerator1")
  (bind _outactors (Actor|GetAllActorsOfClass "/Game/PlayerCharacter.PlayerCharacter_C"))
  (for (_array_element _array_index) _outactors
    (Transformation|SetWorldLocation (Variables|/Game/PlayerCharacter.PlayerCharacter_C|GetCapsule _array_element) (Transformation|GetActorLocation (Utilities|Array|Get(acopy) (Variables|Default|GetPlayerStarts) _array_index)) false true)))

(event Custom|EndAfterDelay
  (Utilities|FlowControl|Delay 1.0)
  (Variables|Default|SetFadeTarget 0.0)
  (Variables|Default|SetState "NewEnumerator2")
  (Audio|Components|Audio|Play (Variables|Default|GetWinSong) 0.0)
  (bind _returnvalue (Actor|GetActorOfClass "/Game/Bogdan/BP_VoiceSystem.BP_VoiceSystem_C"))
  (Audio|Components|Audio|Stop (Variables|/Game/Bogdan/BP_VoiceSystem.BP_VoiceSystem_C|GetSong _returnvalue)))

(event EventBeginPlay
  (Utilities|FlowControl|Sequence
    (:then_0
      (Utilities|FlowControl|Delay 2.0)
      (Variables|Default|SetFadeTarget 0.0)
      (CallFunction|SetupNewGame))
    (:then_1
      (bind _returnvalue (UserInterface|CreateWidget "/Game/Bogdan/WG_IntroScreen.WG_IntroScreen_C"))
      (UserInterface|Viewport|AddtoViewport _returnvalue 0)
      (Variables|Default|SetMenuWidget _returnvalue))))

(event Collision|EventActorBeginOverlap
  (params (OtherActor :type Actor%20Object%20Reference)))

(event EventTick
  (params (DeltaSeconds :type Float%20%28single-precision%29))
  (bind _returnvalue (Game|GetPlayerController 0))
  (Utilities|FlowControl|Sequence
    (:then_0
      (switch Utilities|FlowControl|Switch|SwitchonE_CurrentGameState (Variables|Default|GetState)
        (:NewEnumerator0
          (Game|Player|SetViewTargetwithBlend _returnvalue (Variables|Default|GetPodiumCamera) 0.0 "VTBlend_Linear" 0.0 false))
        (:NewEnumerator1
          (bind _returnvalue_2 (Actor|GetActorOfClass "/Game/ArenaAndCamera.ArenaAndCamera_C"))
          (Game|Player|SetViewTargetwithBlend _returnvalue _returnvalue_2 0.0 "VTBlend_Linear" 0.0 false))))
    (:then_1
      (bind _returnvalue_3 (Class|KismetMathLibrary|FloatSpringInterp (Variables|Default|GetFade) (Variables|Default|GetFadeTarget) (Variables|Default|GetFadeSpring) 0.6 0.5 (* (Utilities|Time|GetWorldDeltaSeconds) 1.0) 0.1 1.0 true 0.0))
      (bind _output_get (Variables|Default|SetFade _returnvalue_3))
      (Rendering|Material|SetScalarParameterValue "/Game/PostProcCollection.PostProcCollection" "Fade" _output_get :!class /Script/Engine.KismetMaterialLibrary))
    (:then_2
      (Widget|SetVisibility (Variables|Default|GetMenuWidget) (Utilities|Select :Index (Variables|Default|GetState) :NewEnumerator0 "Visible" :NewEnumerator1 "Hidden" :NewEnumerator2 "Hidden" :NewEnumerator3 "Hidden" :NewEnumerator4 "Hidden")))))

(fn ConstructionScript)

(fn SetupNewGame
  (Variables|Default|SetState "NewEnumerator0")
  (Audio|Components|Audio|Play (Variables|Default|GetGGJMenu) 0.0)
  (bind _outactors (Actor|GetAllActorsOfClass "/Game/PlayerCharacter.PlayerCharacter_C"))
  (for _array_element _outactors
    (Transformation|SetWorldLocation (Variables|/Game/PlayerCharacter.PlayerCharacter_C|GetCapsule _array_element) (Transformation|GetWorldLocation (Variables|/Game/Bogdan/BP_PlayerPodium.BP_PlayerPodium_C|GetPlayerLoc (Utilities|Array|Get(acopy) (Variables|Default|GetPodiums) (Variables|/Game/PlayerCharacter.PlayerCharacter_C|GetMyControllerIndex _array_element)))) false true)))

(fn BeginMatch
  (Audio|Components|Audio|Stop (Variables|Default|GetGGJMenu))
  (Variables|Default|SetFadeTarget 1.0)
  (Variables|Default|SetState "NewEnumerator3")
  (CallFunction|BeginAfterDelay))

(fn EndMatch
  (Variables|Default|SetFadeTarget 1.0)
  (Variables|Default|SetState "NewEnumerator4")
  (CallFunction|EndAfterDelay))