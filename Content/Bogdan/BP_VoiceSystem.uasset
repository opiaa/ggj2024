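; Voice-input manager that turns the player's speech into spawned word actors during timed windows of the music track.
; Tick starts and stops speech recognition by song segments, streaming captured microphone audio into the recognizer and updating the UI prompt.
; Recognized text is filtered by length and a reject table, shuffled, then queued for interval-based spawning through ArenaAndCamera.
; BeginMusic starts the song and timing; its completion handler ends the match through BP_GameStateManager.
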(event Custom|CustomEvent
  (params (AvailableDevices :type Array%20of%20Audio%20Input%20Device%20Info%20Structures))
  (Variables|Default|SetAudioDevices AvailableDevices)
  (Variables|Default|SetHasBuiltAudioDeviceList true))

(event Custom|OnMusicFinished
  (bind _returnvalue (Actor|GetActorOfClass "/Game/Bogdan/BP_GameStateManager.BP_GameStateManager_C"))
  (Default|EndMatch _returnvalue))

(event Custom|BV_StartingRecog
  (params (bSucceeded :type Boolean))
  (bind _desiredaudiodeviceindex (Variables|Default|GetDesiredAudioDeviceIndex))
  (if bSucceeded
    (bind _returnvalue (Class|CapturableSoundWave|CreateCapturableSoundWave))
    (Variables|Default|SetWave _returnvalue)
    (EventDispatchers|BindEventtoOnPopulateAudioData _returnvalue (delegate Custom|BV_OnPopulate))
    (Class|CapturableSoundWave|StartCapture (Variables|Default|GetWave) _desiredaudiodeviceindex)
    (Development|PrintString (Utilities|String|ToString(Text) (Utilities|Text|FormatText "Audio Device {A}" (.DeviceName (Utilities|Struct|BreakAudioInputDeviceInfo (Utilities|Array|Get(acopy) (Variables|Default|GetAudioDevices) _desiredaudiodeviceindex))))))))

(event Custom|BV_OnPopulate
  (params (PopulatedAudioData :type Array%20of%20Floats%20%28single-precision%29))
  (bind _wave (Variables|Default|GetWave))
  (Class|SpeechRecognizer|ProcessAudioData (Variables|Default|GetRecognizer) PopulatedAudioData (Math|Conversions|ToFloat(Integer) (Class|ImportedSoundWave|GetSampleRate _wave)) (Class|ImportedSoundWave|GetNumOfChannels _wave) false))

(event Custom|EndRecognition
  (Class|CapturableSoundWave|StopCapture (Variables|Default|GetWave))
  (Class|SpeechRecognizer|ForceProcessPendingAudioData (Variables|Default|GetRecognizer)))

(event Custom|BeginRecognition
  (bind _returnvalue (Class|SpeechRecognizer|CreateSpeechRecognizer))
  (bind _output_get (Variables|Default|SetRecognizer _returnvalue))
  (EventDispatchers|BindEventtoOnRecognitionFinished _output_get (delegate Custom|BV_OnRecogFinished))
  (EventDispatchers|BindEventtoOnRecognizedTextSegment (Variables|Default|GetRecognizer) (delegate Custom|BV_Recognized))
  (Class|SpeechRecognizer|SetStreamingDefaults (Variables|Default|GetRecognizer))
  (Class|SpeechRecognizer|SetLanguage (Variables|Default|GetRecognizer) "En")
  (Class|SpeechRecognizer|StartSpeechRecognition (Variables|Default|GetRecognizer) (delegate Custom|BV_StartingRecog)))

(event Custom|BV_OnRecogFinished
  (if (not (Class|CapturableSoundWave|IsCapturing (Variables|Default|GetWave)))
    (Class|SpeechRecognizer|StopSpeechRecognition (Variables|Default|GetRecognizer))
    (Variables|Default|SetRecognizer 0)))

(event Custom|BV_Recognized
  (params (RecognizedWords :type String))
  (if (CallFunction|CheckRecognitionIsValid RecognizedWords)
    (CallFunction|GenerateWords RecognizedWords)))

(event EventBeginPlay
  (Utilities|FlowControl|Sequence
    (:then_0
      (Class|AudioCaptureBlueprintLibrary|GetAvailableAudioInputDevices (delegate Custom|CustomEvent)))
    (:then_3
      (bind _returnvalue (UserInterface|CreateWidget "/Game/VoiceStuff/WG_GameUI.WG_GameUI_C" (Game|GetPlayerController 0)))
      (UserInterface|Viewport|AddtoViewport _returnvalue 0)
      (Variables|Default|SetUIWidget _returnvalue))))

(event Collision|EventActorBeginOverlap
  (params (OtherActor :type Actor%20Object%20Reference)))

(event EventTick
  (params (DeltaSeconds :type Float%20%28single-precision%29))
  (if (Variables|Default|GetRunning)
    (Utilities|FlowControl|Sequence
      (:then_1
        (if (> (- (Utilities|Time|GetGameTimeinSeconds) (Variables|Default|GetTimeLastSpawned)) (Variables|Default|GetTimeBetweenWordSpawns))
          (Utilities|FlowControl|Sequence
            (:then_0
              (if (Utilities|Array|IsNotEmpty (Variables|Default|GetPlsSpawnThese))
                (bind _returnvalue (Actor|GetActorOfClass "/Game/ArenaAndCamera.ArenaAndCamera_C"))
                (Utilities|IsValid _returnvalue
                  (:Is%20Valid
                    (Default|FSpawnWordActor _returnvalue (Utilities|Array|Get(acopy) (Variables|Default|GetPlsSpawnThese)))
                    (Utilities|Array|RemoveIndex (Variables|Default|GetPlsSpawnThese))
                    (Audio|PlaySound2D "/Engine/VREditor/Sounds/UI/Click_on_Button.Click_on_Button" 1.0 1.0 0.0 0 0)))))
            (:then_1
              (Variables|Default|SetTimeLastSpawned (Utilities|Time|GetGameTimeinSeconds))))))
      (:then_2
        (CallFunction|UpdateState))
      (:then_3
        (Variables|/Game/VoiceStuff/WG_GameUI.WG_GameUI_C|SetWantSayStuffPrompt (Variables|Default|GetUIWidget) (Variables|Default|GetDoRecognition))))))

(event Input|KeyboardEvents|T
  (params (Key :type Key%20Structure :default "None"))
  (:Pressed
    (bind _outactors (Actor|GetAllActorsOfClass "/Game/Word_Base.Word_Base_C"))
    (for _array_element _outactors
      (Actor|DestroyActor _array_element))))

(fn ConstructionScript)

(fn GenerateWords
  (params (Text :type String))
  (bind _candidates (LocalVariables|GetCandidates))
  (Utilities|FlowControl|Sequence
    (:then_0
      (for _array_element (Utilities|String|ParseIntoArray Text " ")
        (bind _valid (CallFunction|ValidateWord _array_element))
        (if _valid
          (Utilities|Array|Add (LocalVariables|GetCandidates) _array_element))))
    (:then_1
      (Utilities|Array|Shuffle _candidates)
      (for _index (range 0 (Math|Integer|Min(Integer) (Utilities|Array|LastIndex _candidates) (LocalVariables|GetMaxWordsPerDetection)))
        (Utilities|Array|Add (Variables|Default|GetPlsSpawnThese) (Utilities|Array|Get(acopy) _candidates _index))))))

(fn CheckRecognitionIsValid
  (params (Text :type String))
  (if (or (Utilities|Enum|Equal(Enum) Text " [BLANK_AUDIO]") (Utilities|Enum|Equal(Enum) Text " [Inaudible]"))
    (return false)
    (else
      (return true))))

(fn ValidateWord
  (params (Word :type String))
  (bind _outrownames (DataTable|GetDataTableRowNames "/Game/VoiceStuff/OLDDT_WordRejectTable.OLDDT_WordRejectTable"))
  (for _array_element _outrownames
    (bind _returnvalue (Utilities|GetDataTableRow "/Game/VoiceStuff/OLDDT_WordRejectTable.OLDDT_WordRejectTable" _array_element)
      (:then
        (if (Utilities|Enum|Equal(Enum) (.Text (Utilities|Struct|BreakS_DataString _returnvalue)) Word)
          (return false)))))
  (if (< (Utilities|String|Len Word) 4)
    (return false)
    (else
      (return true))))

(fn UpdateState
  (bind _returnvalue (CallFunction|GetCurrentMusicTime))
  (for _array_element (Variables|Default|GetRecogSegs)
    (if (and (> _returnvalue (.Start (Utilities|Struct|BreakS_TimeSegment _array_element))) (< _returnvalue (.End (Utilities|Struct|BreakS_TimeSegment _array_element))))
      (LocalVariables|SetPleaseIWantToRecognze true)))
  (if (LocalVariables|GetPleaseIWantToRecognze)
    (if (Variables|Default|GetDoRecognition)
      _
      (else
        (CallFunction|BeginRecognition)))
    (Variables|Default|SetDoRecognition true)
    (else
      (if (Variables|Default|GetDoRecognition)
        (CallFunction|EndRecognition))
      (Variables|Default|SetDoRecognition false))))

(fn GetCurrentMusicTime
  (return (- (Utilities|Time|GetGameTimeinSeconds) (Variables|Default|GetTimeMusicStarted))))

(fn BeginMusic
  (bind _song (Variables|Default|GetSong))
  (Variables|Default|SetRunning true)
  (Audio|Components|Audio|Play _song 0.0)
  (Variables|Default|SetTimeMusicStarted (Utilities|Time|GetGameTimeinSeconds))
  (EventDispatchers|BindEventtoOnAudioFinished _song (EventDispatchers|CreateEvent :!event Custom|OnMusicFinished)))